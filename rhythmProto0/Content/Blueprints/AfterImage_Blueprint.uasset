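; AfterImage_Blueprint is an actor that shows a fading afterimage of a character's pose.
; On SpawnImage it creates a dynamic M_AfterImage instance, applies it to the poseable mesh's material slots, and copies the pose from a referenced skeletal mesh component.
; A timeline then drives the material's Opacity parameter and destroys the actor when it finishes.
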(event `SpawnImage`
  (bind _returnvalue (`KismetMaterialLibrary.CreateDynamicMaterialInstance` "/Game/FX/M_AfterImage.M_AfterImage"))
  (set `self.m_afterImageMat` _returnvalue)
  (for _index (range (`PrimitiveComponent.GetNumMaterials` (`self.m_charPose`)))
    (`PrimitiveComponent.SetMaterial` (`self.m_poseableMesh`) _index (`self.m_afterImageMat`)))
  (`PoseableMeshComponent.CopyPoseFromSkeletalComponent` (`self.m_poseableMesh`) (`self.m_charPose`))
  (bind (_direction _opacity) (`Timeline|AfterimageOpacity`)
    (:`Update`
      (`MaterialInstanceDynamic.SetScalarParameterValue` (`self.m_afterImageMat`) "Opacity" _opacity))
    (:`Finished`
      (`self.K2_DestroyActor`))))

(fn `UserConstructionScript`)