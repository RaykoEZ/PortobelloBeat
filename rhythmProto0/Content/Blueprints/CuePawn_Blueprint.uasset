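; Player pawn for a rhythm fighting game, pitting Take's punches and dodges against the DCap enemy.
; Cues forecast each input, and enemy animation callbacks or punch events open and close the timing window, with beat checks in parent-class functions, likely C++.
; Key presses play Take montages, then drive enemy reactions, camera feedback, score updates and success/failure callbacks.
; Also spawns after-images, triggers phase changes and finishes the game with a KO punch.
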(event `self.ReceiveBeginPlay`
  (`PlayerCameraManager.PlayCameraShake` :`self` (`GameplayStatics.GetPlayerCameraManager` 0) :`ShakeClass` "/Game/Anims/Camera/CamShake_Ambient_Blueprint.CamShake_Ambient_Blueprint_C")
  (`KismetSystemLibrary.ExecuteConsoleCommand` "viewmode unlit" null)
  (bind _asbp_anim_dcap (cast `/Game/Anims/DeathCap/New_Placeholders/BP_Anim_DCap` (`SkeletalMeshComponent.GetAnimInstance` (`self.Enemy`))))
  (bind _output_get (set `self.m_animDC` _asbp_anim_dcap))
  (add `/Game/Anims/DeathCap/New_Placeholders/BP_Anim_DCap.InputTriggerNow` _output_get (delegate `beatOn`))
  (add `/Game/Anims/DeathCap/New_Placeholders/BP_Anim_DCap.InputEndsNow` _output_get (delegate `beatOff`))
  (bind _asbp_anim_take (cast `/Game/Anims/Take/New_Placehoders/BP_Anim_Take` (`SkeletalMeshComponent.GetAnimInstance` (`self.Take`))))
  (set `self.m_animTake` _asbp_anim_take))

(event `self.ReceiveTick`
  (params (DeltaSeconds :type "Float (single-precision)"))
  ;[1 1 1] Call to cpp for key press event, subject to optimsation
)

(event `beatOn`
  ;[1 1 1] Call to cpp for key press event, subject to optimsation
  ;;[1 1 1] When input time frame begins
  (`self.onBeatBegin`))

(event `beatOff`
  ;[1 1 1] Call to cpp for key press event, subject to optimsation
  ;;[1 1 1] When input time frame ends
  (`self.setIsFrameOpen` false)
  ;;;[1 1 1] Signals whether this beat has been missed or not
  (bind _returnvalue (`self.endOfInputChecks`))
  (if _returnvalue
    (`self.onDodgeFailed`) ; Edit here for failed input
  )
  (`self.resetState`)
  (set `self.m_currentInput` "NONE")
  (set `self.m_numInput_0` 1)
  (set `/Game/Anims/Take/New_Placehoders/BP_Anim_Take.m_hurt` false (`self.m_animTake`)))

(event `OnCue`
  (params (audioT :type "EInputType Enum" :default "PUNCH") (_i :type Integer))
  ;[1 1 1] Call to cpp for key press event, subject to optimsation
  ;;[1 1 1] Forecast Input
  (bind _output_get (set `self.m_currentInput` audioT))
  (bind _output_get_2 (set `self.m_numInput_0` (`KismetMathLibrary.Conv_IntToByte` _i)))
  (`self.playCue` _output_get _output_get_2))

(event `InputNow`
  ;[1 1 1] Call to cpp for key press event, subject to optimsation
  ;;[1 1 1] Forecast Input
  (`self.setInputIndex` (stale `OnCue` _output_get) (stale `OnCue` _output_get_2)))

(event `PunchNow`
  ;[1 1 1] Call to cpp for key press event, subject to optimsation
  ;;[1 1 1] Forecast Input
  (`self.InputNow`)
  (`self.beatOn`))

(event `PunchEnd`
  ;[1 1 1] Call to cpp for key press event, subject to optimsation
  ;;[1 1 1] Forecast Input
  (`self.beatOff`))

(event `PhaseChange`
  ;[1 1 1] Call to cpp for key press event, subject to optimsation
  (`AnimInstance.Montage_Play` (`self.m_animDC`) "/Game/Anims/DeathCap/New_Placeholders/Anims/AnimMon_DcapPhaseChange_0-1.AnimMon_DcapPhaseChange_0-1" 1.0 "MontageLength" 0.0 true))

(event `OnEndOfGame`
  ;[1 1 1] Call to cpp for key press event, subject to optimsation
  (set `self.m_endOfGame` true))

(event `EndOfGame`
  ;[1 1 1] Call to cpp for key press event, subject to optimsation
  (`self.onGameEnd`)
  (set `self.m_inputEnabled` false)
  (`self.HandleEndOfGame`))

(event `Key|SpaceBar`
  (params (Key :type "Key Structure"))
  (bind _enemy (`self.Enemy`))
  ;[1 1 1] control
  (:`Pressed`
    (if (`self.m_inputEnabled`)
      (`|PlayMontage` (`self.Take`) "/Game/Anims/Take/New_Placehoders/AnimMon_TakeInput.AnimMon_TakeInput" 1.0 0.0 "Punch"
        (:`then`
          (bind _returnvalue (`self.isInputCorrect`))
          (if _returnvalue
            (`|PlayMontage` _enemy "/Game/Anims/DeathCap/New_Placeholders/Anims/AnimMon_DcapTakeDamage.AnimMon_DcapTakeDamage" 1.0 0.0 "TakeDamage"
              (:`then`
                (`self.onPunchSuccess`))
              (:`OnCompleted`
                (`self.EnableInput` null :!label _label)))
            (else
              (`self.onPunchFailed`)
              (`|PlayMontage` _enemy "/Game/Anims/DeathCap/New_Placeholders/Anims/AnimMon_DeathCap_Dodge.AnimMon_DeathCap_Dodge" 1.0 0.0 "Dodge1"
                (:`OnCompleted`
                  (goto _label))))))))))

(event `Key|LeftMouseButton`
  (params (Key :type "Key Structure"))
  ;[1 1 1] control
  (:`Pressed`
    (if (`self.m_inputEnabled`)
      (`|PlayMontage` (`self.Take`) "/Game/Anims/Take/New_Placehoders/AnimMon_TakeInput.AnimMon_TakeInput" 1.0 0.0 "Dodge" :!label _label_2
        (:`then`
          (bind _returnvalue (`self.isInputCorrect`))
          (if _returnvalue
            (`self.onDodgeSuccess`)))))))

(event `Key|Down`
  (params (Key :type "Key Structure"))
  ;[1 1 1] control
  (:`Pressed`
    (goto _label_2)))

(event `AfterImage`
  (bind _returnvalue (`|SpawnActorFromClass` "/Game/Blueprints/AfterImage_Blueprint.AfterImage_Blueprint_C" (`SceneComponent.K2_GetComponentToWorld` (`self.Take`)) "Undefined" "OverrideRootScale" null null))
  (set `/Game/Blueprints/AfterImage_Blueprint.m_charPose` (`self.Take`) _returnvalue)
  (`/Game/Blueprints/AfterImage_Blueprint.SpawnImage` _returnvalue))

(fn `onDodgeFailed`
  (set `/Game/Anims/DeathCap/New_Placeholders/BP_Anim_DCap.m_takeFailed` true (`self.m_animDC`))
  (`self.OnInputFailure`))

(fn `onDodgeSuccess`
  (set `/Game/Anims/DeathCap/New_Placeholders/BP_Anim_DCap.m_playerScore` (`self.getScore`) (`self.m_animDC`))
  (`PlayerCameraManager.PlayCameraAnim` :`self` (`GameplayStatics.GetPlayerCameraManager` 0) :`Anim` "/Game/Anims/Camera/Anim_Camera_Dodge_Success.Anim_Camera_Dodge_Success" :`Duration` 0.3)
  (`self.OnInputSuccess`))

(fn `onPunchFailed`
  (`KismetSystemLibrary.PrintString` "fail")
  (set `/Game/Anims/DeathCap/New_Placeholders/BP_Anim_DCap.m_takeFailed` true (`self.m_animDC`)))

(fn `onPunchSuccess`
  (bind _m_animdc (`self.m_animDC`))
  (if (`self.m_endOfGame`)
    (`AnimInstance.Montage_Play` (`self.m_animDC`) "/Game/Anims/DeathCap/New_Placeholders/Anims/AnimMon_DcapKO.AnimMon_DcapKO" 1.0 "MontageLength" 0.0 true)
    (`self.EndOfGame`)
    (`self.DisableInput` null)
    (else
      (`KismetSystemLibrary.PrintString` "Succ")
      (set `/Game/Anims/DeathCap/New_Placeholders/BP_Anim_DCap.m_takeFailed` false _m_animdc)
      (set `/Game/Anims/DeathCap/New_Placeholders/BP_Anim_DCap.m_hurt` true _m_animdc)
      (set `/Game/Anims/DeathCap/New_Placeholders/BP_Anim_DCap.m_numHurt` (+ (`/Game/Anims/DeathCap/New_Placeholders/BP_Anim_DCap.m_numHurt` _m_animdc) 1) _m_animdc)
      (set `/Game/Anims/DeathCap/New_Placeholders/BP_Anim_DCap.m_playerScore` (`self.getScore`) _m_animdc)
      (`PlayerCameraManager.PlayCameraShake` :`self` (`GameplayStatics.GetPlayerCameraManager` 0) :`ShakeClass` "/Game/Anims/Camera/CamShake_Punch_Success_Streak_Blueprint.CamShake_Punch_Success_Streak_Blueprint_C")
      (`self.OnInputSuccess`))))

(fn `UserConstructionScript`)