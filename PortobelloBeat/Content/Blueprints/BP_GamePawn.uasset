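; Player pawn for a beat-timed boxing game where Take punches and dodges the enemy DCap.
; Enemy animation dispatchers and punch events open and close input windows, while functions not defined here, likely native, judge correctness and score.
; Cooldown-gated punch and dodge keys play montage variations, with results driving animation flags, face textures and camera effects.
; It also owns the menu widgets, pause, phase-change cinematics, score-gated final punch and restart reset.
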(event `self.ReceiveBeginPlay`
  (add `/Game/UI/UI_Endgame.OnRestartGame` (`self.m_endGameUI`) (delegate `RestartGame`))
  (add `/Game/UI/UI_Pause.OnRestartGame` (`self.m_pauseMenu`) (delegate `RestartGame`))
  (`self.displayUI` (`self.m_mainMenu`))
  (`PlayerCameraManager.PlayCameraShake` :`self` (`GameplayStatics.GetPlayerCameraManager` 0) :`ShakeClass` "/Game/Anims/Camera/CamShake_Ambient.CamShake_Ambient_C")
  (`KismetSystemLibrary.ExecuteConsoleCommand` "viewmode unlit" null)
  (bind _asbp_anim_dcap (cast `/Game/Anims/DeathCap/New_Placeholders/BP_Anim_DCap` (`SkeletalMeshComponent.GetAnimInstance` (`self.Enemy`))))
  (bind _output_get (set `self.m_animDC` _asbp_anim_dcap))
  (add `/Game/Anims/DeathCap/New_Placeholders/BP_Anim_DCap.InputTriggerNow` _output_get (delegate `beatOn`))
  (add `/Game/Anims/DeathCap/New_Placeholders/BP_Anim_DCap.InputEndsNow` _output_get (delegate `beatOff`))
  (bind _asbp_anim_take (cast `/Game/Anims/Take/New_Placehoders/BP_Anim_Take` (`SkeletalMeshComponent.GetAnimInstance` (`self.Take`))))
  (set `self.m_animTake` _asbp_anim_take)
  (`self.FinishedBPInit`))

(event `beatOn`
  ;[1 1 1] Call to cpp for key press event, subject to optimsation
  ;;[1 1 1] When input time frame begins
  (`self.onBeatBegin`))

(event `RestartGame`
  (bind _m_animdc (`self.m_animDC`))
  ;[1 1 1] UI Events
  (`self.setIsFinalPunch` false)
  (`self.resetStates_BP`)
  (`/Game/Anims/Take/New_Placehoders/BP_Anim_Take.ResetStates` (`self.m_animTake`))
  (`/Game/Anims/DeathCap/New_Placeholders/BP_Anim_DCap.ResetStates` _m_animdc)
  (set `/Game/Anims/DeathCap/New_Placeholders/BP_Anim_DCap.m_victory` false _m_animdc))

(event `OnResultScreen`
  (bind _m_endgameui (`self.m_endGameUI`))
  ;[1 1 1] UI Events
  (`UserWidget.PlayAnimation` _m_endgameui (`/Game/UI/UI_Endgame.FadeIn` _m_endgameui) 0.0 1 "Forward" 1.0)
  (`self.displayUI` _m_endgameui))

(event `beatOff`
  ;[1 1 1] Call to cpp for key press event, subject to optimsation
  ;;[1 1 1] When input time frame ends
  (`self.setIsFrameOpen` false)
  ;;;[1 1 1] Signals whether this beat has been missed or not
  (bind _returnvalue (`self.endOfInputChecks`))
  (if _returnvalue
    (`self.onDodgeFailed`) ; Edit here for failed input
  )
  (`self.endOfBeatCleanup`))

(event `OnCue`
  (params (audioT :type "EInputType Enum" :default "PUNCH") (_i :type Integer))
  ;[1 1 1] Call to cpp for key press event, subject to optimsation
  ;;[1 1 1] Forecast Input
  (bind _output_get (set `self.m_currentInput` audioT))
  (bind _output_get_2 (set `self.m_numInput_0` (`KismetMathLibrary.Conv_IntToByte` _i)))
  (`self.playCue` _output_get _output_get_2))

(event `InputNow`
  ;[1 1 1] Call to cpp for key press event, subject to optimsation
  ;;[1 1 1] Forecast Input
  (`self.setInputIndex` (stale `OnCue` _output_get) (stale `OnCue` _output_get_2)))

(event `PunchNow`
  ;[1 1 1] Call to cpp for key press event, subject to optimsation
  ;;[1 1 1] Forecast Input
  (`self.InputNow`)
  (`self.beatOn`))

(event `PunchEnd`
  ;[1 1 1] Call to cpp for key press event, subject to optimsation
  ;;[1 1 1] Forecast Input
  (`self.beatOff`))

(event `PhaseChange`
  (params (_isPlayer :type Boolean))
  (bind _returnvalue (`GameplayStatics.GetPlayerController` 0))
  ;[1 1 1] Call to cpp for key press event, subject to optimsation
  (`self.DisableInput` _returnvalue)
  (`self.M_PhaseShift` _isPlayer)
  (`self.EnableInput` _returnvalue))

(event `OnEndOfGame`
  ;[1 1 1] Call to cpp for key press event, subject to optimsation
  (bind _output_get (set `self.m_endOfGame` true))
  (`self.setIsFinalPunch` _output_get)
  (`self.PreEndOfGame`)
  (`PlayerCameraManager.PlayCameraAnim` :`self` (`GameplayStatics.GetPlayerCameraManager` 0) :`Anim` "/Game/Anims/Camera/Anim_Camera_Take_Final_Punch.Anim_Camera_Take_Final_Punch"))

(event `EndOfGame`
  ;[1 1 1] Call to cpp for key press event, subject to optimsation
  (`self.onGameEnd`)
  (set `self.m_inputEnabled` false)
  (`/Game/UI/UI_Endgame.setupResultPage` (`self.m_endGameUI`))
  (`self.HandleEndOfGame`))

(event `OnFinalPunch`
  ;[1 1 1] Call to cpp for key press event, subject to optimsation
  (set `/Game/Anims/Take/New_Placehoders/BP_Anim_Take.m_punchSwitch` true (`self.m_animTake`))
  (`self.onGameEnd`))

(event `Key|SpaceBar`
  (params (Key :type "Key Structure"))
  ;[1 1 1] control
  (:`Pressed`
    (`self.M_CheckDodgeLock`)
    (`self.checkInputCD`)
    (`/Engine/EditorBlueprintResources/StandardMacros.DoOnce` false :!label _label
      (:`Completed`
        (`self.M_PunchVariation`)
        (bind _returnvalue (`self.isInputCorrect`))
        (if _returnvalue
          (set `self.c_punchSwitch` (not (`self.c_punchSwitch`)))
          (`self.onPunchSuccess`)
          (else
            (`self.onPunchFailed`)))))))

(event `Key|LeftMouseButton`
  (params (Key :type "Key Structure"))
  ;[1 1 1] control
  (:`Pressed`
    (`self.M_CheckPunchLock` :!label _label_2)
    (`self.checkInputCD`)
    (`/Engine/EditorBlueprintResources/StandardMacros.DoOnce` false :!label _label_3
      (:`Completed`
        (`self.M_DodgeVariation`)
        (bind _returnvalue (`self.isInputCorrect`))
        (if _returnvalue
          (`self.onDodgeSuccess`))))))

(event `Key|Down`
  (params (Key :type "Key Structure"))
  ;[1 1 1] control
  (:`Pressed`
    (goto _label_2)))

(event `InputCooldownTimer`
  ;[1 1 1] control
  (`KismetSystemLibrary.K2_SetTimerDelegate` (delegate `EnableInputNow`) (`self.m_inputCD`))
  (set `self.m_inputEnabled` false))

(event `EnableInputNow`
  ;[1 1 1] control
  (set `self.m_inputEnabled` true)
  (`|ExecutionSequence`
    (:`then_0`
      (goto _label :!via `Reset`))
    (:`then_1`
      (goto _label_3 :!via `Reset`))))

(event `Key|Q`
  (params (Key :type "Key Structure"))
  ;[1 1 1] control
  (:`Released`
    (if (not (`self.m_noMoreInput`))
      (`self.OnPauseGame`)
      (`self.displayUI` (`self.m_pauseMenu`))
      (`GameplayStatics.SetGamePaused` true))))

(event `AfterImage`
  (bind _returnvalue (`|SpawnActorFromClass` "/Game/Blueprints/AfterImage_Blueprint.AfterImage_Blueprint_C" (`SceneComponent.K2_GetComponentToWorld` (`self.Take`)) "Undefined" "OverrideRootScale" null null))
  (set `/Game/Blueprints/AfterImage_Blueprint.m_charPose` (`self.Take`) _returnvalue)
  (`/Game/Blueprints/AfterImage_Blueprint.SpawnImage` _returnvalue))

(fn `checkGameWon`
  (returns (ReturnValue :type Boolean))
  (return (>= (`self.getScore`) (`self.m_clearMargin`))))

(fn `checkInputCD`
  (if (`self.m_inputEnabled`)
    (`self.InputCooldownTimer`)
    (return)))

(fn `displayUI`
  (params (_show :type "UserWidget Object Reference"))
  (`UserWidget.AddToViewport` _show 0)
  (set `PlayerController.bShowMouseCursor` true (`GameplayStatics.GetPlayerController` 0)))

(fn `endOfBeatCleanup`
  (`self.resetState`)
  (if (and (== (`self.m_numInput_0`) 1) (not (`self.c_punchSwitch`)))
    ;[1 1 1] If we are punching once, force reset to let us do Punch1 next time
    (set `self.c_punchSwitch` true))
  (set `self.m_currentInput` "NONE")
  (set `self.m_numInput_0` 1))

(fn `initUI`
  (bind _returnvalue (`GameplayStatics.GetPlayerController` 0))
  (bind _returnvalue_2 (`|CreateWidget` "/Game/UI/UI_Main.UI_Main_C" _returnvalue))
  (set `self.m_mainMenu` _returnvalue_2)
  (bind _returnvalue_3 (`|CreateWidget` "/Game/UI/UI_Pause.UI_Pause_C" _returnvalue))
  (set `self.m_pauseMenu` _returnvalue_3)
  (bind _returnvalue_4 (`|CreateWidget` "/Game/UI/UI_Gameplay.UI_Gameplay_C" _returnvalue))
  (set `self.m_gameplayUI` _returnvalue_4)
  (bind _returnvalue_5 (`|CreateWidget` "/Game/UI/UI_Endgame.UI_Endgame_C" _returnvalue))
  (set `self.m_endGameUI` _returnvalue_5))

(fn `onDodgeFailed`
  (if (`self.m_endOfGame`)
    (set `self.m_noMoreInput` true)
    (else
      (`self.OnInputFailure`))))

(fn `onDodgeSuccess`
  (if (`self.m_endOfGame`)
    (set `self.m_noMoreInput` true)
    (else
      (`PlayerCameraManager.PlayCameraAnim` :`self` (`GameplayStatics.GetPlayerCameraManager` 0) :`Anim` "/Game/Anims/Camera/Anim_Camera_Dodge_Success.Anim_Camera_Dodge_Success" :`Duration` 0.3)
      (`MaterialInstanceDynamic.SetTextureParameterValue` (`self.m_takeFace`) "Expression" "/Game/Textures/shitake_textures/Faces/shitake_dodge_mask.shitake_dodge_mask")
      (`self.OnInputSuccess`))))

(fn `onPunchFailed`
  (if (`self.m_endOfGame`)
    (set `self.m_noMoreInput` true)
    (else
      (`AnimInstance.Montage_Play` (`self.m_animTake`) "/Game/Anims/Take/New_Placehoders/Anims/Montages/AnimMon_Take_Punch1_Fail.AnimMon_Take_Punch1_Fail" 1.0 "MontageLength" 0.0 true)
      (set `/Game/Anims/DeathCap/New_Placeholders/BP_Anim_DCap.m_takeFailed` true (`self.m_animDC`)))))

(fn `onPunchSuccess`
  (bind _m_animdc (`self.m_animDC`))
  (if (and (`self.m_endOfGame`) (`self.checkGameWon`))
    (`PlayerCameraManager.PlayCameraAnim` :`self` (`GameplayStatics.GetPlayerCameraManager` 0) :`Anim` "/Game/Anims/Camera/Anim_Camera_KO_Charge.Anim_Camera_KO_Charge")
    (set `/Game/Anims/Take/New_Placehoders/BP_Anim_Take.m_finalPunch` true (`self.m_animTake`))
    (set `self.m_noMoreInput` true)
    (`self.OnFinalCharge`)
    (else
      (set `/Game/Anims/DeathCap/New_Placeholders/BP_Anim_DCap.m_takeFailed` false _m_animdc)
      (set `/Game/Anims/DeathCap/New_Placeholders/BP_Anim_DCap.m_hurt` true _m_animdc)
      (`/Engine/EditorBlueprintResources/StandardMacros.IncrementInt` (`/Game/Anims/DeathCap/New_Placeholders/BP_Anim_DCap.m_numHurt` _m_animdc)
        (:`  `
          (`PlayerCameraManager.PlayCameraShake` :`self` (`GameplayStatics.GetPlayerCameraManager` 0) :`ShakeClass` "/Game/Anims/Camera/CamShake_Punch_Success_Streak.CamShake_Punch_Success_Streak_C")
          (`self.OnInputSuccess`))))))

(fn `resetStates_BP`
  (`self.resetScore`)
  (set `self.m_inputEnabled` true)
  (set `self.m_noMoreInput` false)
  (set `self.m_endOfGame` false)
  (`MaterialInstanceDynamic.SetTextureParameterValue` (`self.m_dCapFace`) "Expression" "/Game/Anims/DeathCap/New_Placeholders/dcap_face_mask_idle.dcap_face_mask_idle"))

(fn `UserConstructionScript`
  (bind _returnvalue (`PrimitiveComponent.CreateDynamicMaterialInstance` (`self.shitake_face_mesh`) 0 "/Game/Textures/shitake_textures/Faces/Take_Faces.Take_Faces" "None"))
  (set `self.m_takeFace` _returnvalue)
  (bind _returnvalue_2 (`PrimitiveComponent.CreateDynamicMaterialInstance` (`self.dcap_face_mesh`) 0 "/Game/Textures/deathcap_textures/Faces/dcap_face_mask_idle_Mat.dcap_face_mask_idle_Mat" "None"))
  (set `self.m_dCapFace` _returnvalue_2)
  (`self.initUI`))